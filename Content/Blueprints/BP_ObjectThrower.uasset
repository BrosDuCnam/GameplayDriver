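; BP_ObjectThrower spawns and launches BP_Ball actors in response to "throw_object" socket events from the game instance's SIO client.
; On BeginPlay it binds that event to ThrowObject, which reads JSON location and velocity arrays.
; Location's second and third components scale across a Width by Height plane along forward and up; velocity becomes an actor-relative, mass-independent impulse.
; Tick draws debug edges of that plane and the actor's axes.
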(event `self.ReceiveTick`
  (params (DeltaSeconds :type "Float (single-precision)"))
  (bind _returnvalue (`self.K2_GetActorLocation`))
  (bind _returnvalue_2 (`self.K2_GetActorLocation`))
  (bind _returnvalue_3 (`self.K2_GetActorLocation`))
  (bind _returnvalue_4 (`self.K2_GetActorLocation`))
  (bind _height (`self.height`))
  (bind _width (`self.width`))
  (bind _returnvalue_5 (* (`self.GetActorForwardVector`) (`KismetMathLibrary.MakeVector` _width _width _width)))
  (bind _returnvalue_6 (* (`self.GetActorUpVector`) (`KismetMathLibrary.MakeVector` _height _height _height)))
  (bind _returnvalue_7 (+ _returnvalue_2 (+ _returnvalue_5 _returnvalue_6)))
  ;[1 0 0] Debug Box Thrower
  (if (`self.ActivateDebugLine`)
    (`KismetSystemLibrary.DrawDebugLine` (+ _returnvalue_2 _returnvalue_5) _returnvalue_7 (struct :`R` 0.25 :`B` 0.196448 :`A` 1.0) 0.0 10.0)
    (`KismetSystemLibrary.DrawDebugLine` _returnvalue_7 (+ _returnvalue_2 _returnvalue_6) (struct :`R` 0.25 :`B` 0.196448 :`A` 1.0) 0.0 10.0)
    (`KismetSystemLibrary.DrawDebugArrow` _returnvalue_4 (+ _returnvalue_4 (* (`self.GetActorForwardVector`) (1000.0 1000.0 1000.0))) 0.0 (struct :`R` 0.635417 :`B` 0.025695 :`A` 1.0) 0.0 10.0)
    (`KismetSystemLibrary.DrawDebugArrow` _returnvalue_3 (+ _returnvalue_3 (* (`self.GetActorRightVector`) (1000.0 1000.0 1000.0))) 0.0 (struct :`G` 0.427083 :`B` 0.051806 :`A` 1.0) 0.0 10.0)
    (`KismetSystemLibrary.DrawDebugArrow` _returnvalue (+ _returnvalue (* (`self.GetActorUpVector`) (1000.0 1000.0 1000.0))) 0.0 (struct :`G` 0.063085 :`B` 0.427083 :`A` 1.0) 0.0 10.0)))

(event `self.ReceiveBeginPlay`
  (set `self.ActivateDebugLine` true)
  (set `self.velocityScale` 1.0)
  (set `self.height` 150.0)
  (set `self.width` 400.0)
  (`SocketIOClientComponent.BindEventToDelegate` (`/Game/Blueprints/BP_Client.SIOClient` (`/Game/Blueprints/BP_GameInstance.Client` (cast `/Game/Blueprints/BP_GameInstance` (`GameplayStatics.GetGameInstance`) :!pure true))) "throw_object" (delegate `ThrowObject`) "/" "USE_DEFAULT"))

(event `ThrowObject`
  (params (EventData :type "SIOJsonValue Object Reference"))
  (bind _returnvalue (`SIOJLibrary.Conv_JsonValueToJsonObject` EventData))
  (bind _velocityscale (`self.velocityScale`))
  (`KismetSystemLibrary.PrintString` "TEST THROW" true true (struct :`G` 0.66 :`B` 1.0 :`A` 1.0) 10.0)
  (bind _returnvalue_2 (`SIOJsonObject.GetNumberArrayField` _returnvalue "location"))
  (bind _returnvalue_3 (`SIOJsonObject.GetNumberArrayField` _returnvalue "velocity"))
  (bind _returnvalue_4 (* (`|GetArrayItem` _returnvalue_2 1) (`self.width`)))
  (bind _returnvalue_5 (* (`|GetArrayItem` _returnvalue_2 2) (`self.height`)))
  (bind _returnvalue_6 (`|SpawnActorFromClass` "/Game/Blueprints/Thrower/BP_Ball.BP_Ball_C" (`KismetMathLibrary.Conv_VectorToTransform` (+ (`self.K2_GetActorLocation`) (+ (* (`KismetMathLibrary.MakeVector` _returnvalue_4 _returnvalue_4 _returnvalue_4) (`self.GetActorForwardVector`)) (* (`KismetMathLibrary.MakeVector` _returnvalue_5 _returnvalue_5 _returnvalue_5) (`self.GetActorUpVector`))))) "Undefined" "OverrideRootScale" null null))
  (bind _returnvalue_7 (* (`|GetArrayItem` _returnvalue_3) _velocityscale))
  (bind _returnvalue_8 (* (`|GetArrayItem` _returnvalue_3 1) _velocityscale))
  (bind _returnvalue_9 (* (`|GetArrayItem` _returnvalue_3 2) _velocityscale))
  (`PrimitiveComponent.AddImpulse` (`/Game/Blueprints/Thrower/BP_Ball.Sphere` _returnvalue_6) (+ (* (`KismetMathLibrary.MakeVector` _returnvalue_7 _returnvalue_7 _returnvalue_7) (`self.GetActorForwardVector`)) (* (`KismetMathLibrary.MakeVector` _returnvalue_8 _returnvalue_8 _returnvalue_8) (`self.GetActorRightVector`)) (* (`KismetMathLibrary.MakeVector` _returnvalue_9 _returnvalue_9 _returnvalue_9) (`self.GetActorUpVector`))) "None" true))

(fn `UserConstructionScript`)