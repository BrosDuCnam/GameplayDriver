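; BP_Client is a Socket.IO client that opens a connection to a server when play begins.
; On BeginPlay it registers itself as the Client on BP_GameInstance, then calls Connect.
; Connect builds an HTTP address from the Ip and Port variables and connects the SIOClient component, passing Type as a "type" parameter in the URL params.
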(event `self.ReceiveBeginPlay`
  (set `/Game/Blueprints/BP_GameInstance.Client` self (cast `/Game/Blueprints/BP_GameInstance` (`GameplayStatics.GetGameInstance`) :!pure true))
  (`self.Connect`))

(fn `BuildURL`
  (returns (url :type String))
  (return (`KismetStringLibrary.Concat_StrStr` "http://" (`self.Ip`) ":" (`self.Port`))))

(fn `Connect`
  (bind _output_get (set `SocketIOClientComponent.URLParams` (make `SIOConnectParams` (`self.BuildURL`) _ (`|MakeMap` "type" (`self.Type`))) (`self.SIOClient`)))
  (`SocketIOClientComponent.ConnectWithParams` (`self.SIOClient`) _output_get))

(fn `UserConstructionScript`)